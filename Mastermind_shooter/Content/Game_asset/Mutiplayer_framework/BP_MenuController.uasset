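; Player controller for the multiplayer menu and lobby, giving the local player a UI-only cursor and a lobby widget.
; Initial setup loads the player profile from a local save slot, creating it if missing, then passes it through ServerUpdateLobby to BP_MainMenu_gamemod to refresh the lobby.
; UpdatePlayersName rebuilds the widget's name list from supplied profiles.
; EndClientSession destroys the session and returns to the main menu.
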(event `self.ReceiveBeginPlay`
  (if (`self.IsLocalController`)
    (set `self.bShowMouseCursor` true)
    (`WidgetBlueprintLibrary.SetInputMode_UIOnlyEx` self null)))

(event `EndClientSession`
  (`DestroySessionCallbackProxy.DestroySession` self
    (:`then`
      (`GameplayStatics.OpenLevelBySoftObjectPtr` "/Game/Game_asset/RealLevels/Levels/Menu/MainMenu.MainMenu"))))

(event `CreateLobbyMenu`
  (`self.UI_ShowLobbyMenu`))

(event `Initial_Setup`
  (`self.LoadSaveProfiled`)
  (`self.Server_UpdateLobby` (`self.Player Profile`)))

(event `Server_UpdateLobby`
  (params (`Player Profile` :type "/Game/Game_asset/Mutiplayer_framework/SavedData/S_PlayerProfile Structure"))
  (set `self.Player Profile` `Player Profile`)
  (bind _asbp_main_menu_gamemod (cast `/Game/Game_asset/RealLevels/Levels/Menu/BP_MainMenu_gamemod` (`GameplayStatics.GetGameMode`)))
  (`/Game/Game_asset/RealLevels/Levels/Menu/BP_MainMenu_gamemod.UpdateLobby` _asbp_main_menu_gamemod true))

(event `UpdatePlayersName`
  (params (PlayerProfiles :type "Array of /Game/Game_asset/Mutiplayer_framework/SavedData/S_PlayerProfile Structure"))
  (bind _wb_lobbymenu (`self.WB_LobbyMenu`))
  (`/Engine/EditorBlueprintResources/StandardMacros.IsValid` _wb_lobbymenu
    (:`Is Valid`
      (`/Game/Game_asset/RealLevels/Levels/Menu/WidgetMenu/WB_LobbyMenu.ClearPlayersName` _wb_lobbymenu)
      (`/Game/Game_asset/RealLevels/Levels/Menu/WidgetMenu/WB_LobbyMenu.UpdatePlayersName` _wb_lobbymenu PlayerProfiles))))

(fn `LoadSaveProfiled`
  (bind _returnvalue (`GameplayStatics.DoesSaveGameExist` (`self.Local Slot Name`)))
  (if (not _returnvalue)
    (bind _returnvalue_2 (`GameplayStatics.CreateSaveGameObject` "/Game/Game_asset/Mutiplayer_framework/SavedData/SG_PlayerProfile.SG_PlayerProfile_C"))
    (`GameplayStatics.SaveGameToSlot` _returnvalue_2 (`self.Local Slot Name`)))
  (bind _returnvalue_3 (`GameplayStatics.LoadGameFromSlot` (`self.Local Slot Name`)))
  (bind _assg_player_profile (cast `/Game/Game_asset/Mutiplayer_framework/SavedData/SG_PlayerProfile` _returnvalue_3))
  (set `self.Player Profile` (`/Game/Game_asset/Mutiplayer_framework/SavedData/SG_PlayerProfile.PlayerProfile` _assg_player_profile))
  (return))

(fn `UI_ShowLobbyMenu`
  (`/Engine/EditorBlueprintResources/StandardMacros.IsValid` (`self.WB_LobbyMenu`)
    (:`Is Valid`
      _)
    (:`Is Not Valid`
      (bind _returnvalue (`|CreateWidget` "/Game/Game_asset/RealLevels/Levels/Menu/WidgetMenu/WB_LobbyMenu.WB_LobbyMenu_C" self))
      (set `self.WB_LobbyMenu` _returnvalue)))
  (`UserWidget.AddToViewport` (`self.WB_LobbyMenu`) 0)
  (return))

(fn `UserConstructionScript`)