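; BP_MainMenu_gamemod is the menu game mode that registers players joining the lobby and keeps their profile lists in sync.
; When a player starts on the Lobby Menu Map, it stores their BP_MenuController and tells it to create the lobby menu and run initial setup.
; UpdateLobby, gated by a PlayerNames flag, rebuilds the profile list from all stored controllers and sends it to each to update player names.
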(event `self.HandleStartingNewPlayer`
  (params (NewPlayer :type "PlayerController Object Reference"))
  (bind _returnvalue (`GameplayStatics.GetCurrentLevelName` true))
  (switch `string` _returnvalue
    (:`LobbyMenuMap`
      (bind _asbp_menu_controller (cast `/Game/Game_asset/Mutiplayer_framework/BP_MenuController` NewPlayer))
      (`KismetArrayLibrary.Array_Add` (`self.All_ConnectedPlayers`) _asbp_menu_controller)
      (`/Game/Game_asset/Mutiplayer_framework/BP_MenuController.CreateLobbyMenu` _asbp_menu_controller)
      (`/Game/Game_asset/Mutiplayer_framework/BP_MenuController.Initial_Setup` _asbp_menu_controller))))

(event `UpdateLobby`
  (params (PlayerNames :type Boolean))
  (if PlayerNames
    (`KismetArrayLibrary.Array_Clear` (`self.All_PlayerProfiles`))
    (for _array_element (`self.All_ConnectedPlayers`)
      (`KismetArrayLibrary.Array_Add` (`self.All_PlayerProfiles`) (`/Game/Game_asset/Mutiplayer_framework/BP_MenuController.Player Profile` _array_element)))
    (for _array_element_2 (`self.All_ConnectedPlayers`)
      (if PlayerNames
        (`/Game/Game_asset/Mutiplayer_framework/BP_MenuController.UpdatePlayersName` _array_element_2 (`self.All_PlayerProfiles`))))))

(fn `UserConstructionScript`)