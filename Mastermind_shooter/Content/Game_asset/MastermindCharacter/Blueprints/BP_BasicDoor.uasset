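; BP_BasicDoor is a two-panel sliding door whose left and right panels open and close independently through separate toggle events.
; Each toggle flips its panel's open state and slides it a fixed distance along relative X with an eased one-second MoveComponentTo, then prints the new state.
; A single completion flag shared by both panels ignores any toggle while either is moving.
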(event `ToggleDoorRight`
  (bind _rdoor (`self.RDoor`))
  (bind _relativelocation (`SceneComponent.RelativeLocation` (`self.RDoor`)))
  (if (`self.b_MoveCompleted`)
    (if (`self.b_isOpen_Right`)
      (bind _output_get (set `self.v_TargetLocation` _relativelocation))
      (set `self.b_isOpen_Right` false)
      (set `self.b_MoveCompleted` false)
      (`KismetSystemLibrary.MoveComponentTo` _rdoor (+ _output_get (225.0 0.0 0.0)) (struct) true true 1.0)
      (set `self.b_MoveCompleted` true)
      (`KismetSystemLibrary.PrintText` "Right Door Close")
      (else
        (bind _output_get_2 (set `self.v_TargetLocation` _relativelocation))
        (set `self.b_isOpen_Right` true)
        (set `self.b_MoveCompleted` false)
        (`KismetSystemLibrary.MoveComponentTo` _rdoor (- _output_get_2 (225.0 0.0 0.0)) (struct) true true 1.0)
        (set `self.b_MoveCompleted` true)
        (`KismetSystemLibrary.PrintText` "Right Door Open")))))

(event `ToggleDoorLeft`
  (bind _ldoor (`self.LDoor`))
  (bind _relativelocation (`SceneComponent.RelativeLocation` (`self.LDoor`)))
  (if (`self.b_MoveCompleted`)
    (if (`self.b_isOpen_Left`)
      (bind _output_get (set `self.v_TargetLocation` _relativelocation))
      (set `self.b_isOpen_Left` false)
      (set `self.b_MoveCompleted` false)
      (`KismetSystemLibrary.MoveComponentTo` _ldoor (+ _output_get (225.0 0.0 0.0)) (struct) true true 1.0)
      (set `self.b_MoveCompleted` true)
      (`KismetSystemLibrary.PrintText` "Left Door Close")
      (else
        (bind _output_get_2 (set `self.v_TargetLocation` _relativelocation))
        (set `self.b_isOpen_Left` true)
        (set `self.b_MoveCompleted` false)
        (`KismetSystemLibrary.MoveComponentTo` _ldoor (- _output_get_2 (225.0 0.0 0.0)) (struct) true true 1.0)
        (set `self.b_MoveCompleted` true)
        (`KismetSystemLibrary.PrintText` "Left Door Open")))))

(fn `UserConstructionScript`)